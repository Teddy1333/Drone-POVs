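; BP_HUD_BaseSetup is an actor Blueprint that sets up the drone HUD widgets when play begins.
; BeginPlay sets game-only input on the owning player controller, then creates a HUD widget and adds it to the viewport.
; It also creates a WB_Drone_HUD instance as the camera menu and stores it in an array without displaying it.
; A RemoveFromParent call on the HUD is left unconnected.
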(event `self.ReceiveBeginPlay`
  ;[1 1 1] Focus input on game
  (`WidgetBlueprintLibrary.SetInputMode_GameOnly` (`self.GetOwningPlayerController`))
  ;[1 1 1] View
  (bind _returnvalue (`|CreateWidget` "/Game/WB_Drone_HUD.WB_Drone_HUD_C" (`self.GetOwningPlayerController`)))
  (bind _output_get (set `self.WB_Drone_HUD` _returnvalue))
  (`UserWidget.AddToViewport` _output_get 0)
  ;[1 1 1] View Menu
  (bind _returnvalue_2 (`|CreateWidget` "/Game/WB_Drone_HUD.WB_Drone_HUD_C" (`self.GetOwningPlayerController`)))
  (bind _output_get_2 (set `self.WB_CameraMenu` _returnvalue_2))
  (`KismetArrayLibrary.Array_Add` (`|MakeArray` (`self.ArrayList`)) _output_get_2))

(fn `UserConstructionScript`)